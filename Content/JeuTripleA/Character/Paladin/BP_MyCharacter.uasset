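; Player character Blueprint in the Paladin folder that drives the HUD, item use, death handling and targeting.
; BeginPlay creates the HUD with health and portrait; Tick refreshes the held item's icon and count from the GameInstance inventory.
; Health updates set death at zero; an update while dead resets game completion, then loads MenuMap after a delay.
; Box overlaps, both begin and end, write MTarget on the MyCharacter found via GetActorOfClass.
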(event `self.ReceiveBeginPlay`
  (bind _returnvalue (`|GenericCreateObject` "/Game/JeuTripleA/Character/Paladin/Anims/Ui/WBP_PlayerHUD.WBP_PlayerHUD_C" (`GameplayStatics.GetPlayerController` 0)))
  (bind _output_get (set `self.ThePlayerHUD` _returnvalue))
  (`UserWidget.AddToViewport` _output_get 0)
  (bind _returnvalue_2 (`self.GetPercentHealth`))
  (`ProgressBar.SetPercent` (`/Game/JeuTripleA/Character/Paladin/Anims/Ui/WBP_PlayerHUD.HP` (`self.ThePlayerHUD`)) _returnvalue_2)
  (bind _returnvalue_3 (`self.GetPortrait`))
  (`Image.SetBrushFromTexture` (`/Game/JeuTripleA/Character/Paladin/Anims/Ui/WBP_PlayerHUD.Portrait` (`self.ThePlayerHUD`)) _returnvalue_3 false)
  (bind _asmy_character (cast `MyCharacter` (`self.GetController`)))
  (bind _output_get_2 (set `self.TheController` _asmy_character))
  (`PlayerController.SetAudioListenerAttenuationOverride` _output_get_2 (`self.Mesh`) (0.0 0.0 0.0)))

(event `self.OnUpdateHealth`
  (bind _returnvalue (`GameplayStatics.GetActorOfClass` "/Script/MyProject.MyCharacter"))
  (if (`MyCharacter.IsDead` _returnvalue)
    (bind _asmy_game_instance (cast `MyGameInstance` (`GameplayStatics.GetGameInstance`)))
    (`MyGameInstance.ResetGameCompletion` _asmy_game_instance)
    (`KismetSystemLibrary.Delay` 4.0)
    (`GameplayStatics.OpenLevel` "MenuMap")
    (else
      (bind _returnvalue_2 (`self.GetPercentHealth`))
      (`ProgressBar.SetPercent` (`/Game/JeuTripleA/Character/Paladin/Anims/Ui/WBP_PlayerHUD.HP` (`self.ThePlayerHUD`)) _returnvalue_2)
      (bind _returnvalue_3 (`self.GetHealth`))
      (if (<= _returnvalue_3 0.0)
        (bind _returnvalue_4 (`GameplayStatics.GetActorOfClass` "/Script/MyProject.MyCharacter"))
        (`MyCharacter.SetDead` _returnvalue_4)))))

(event `InputAction|Use`
  (params (Key :type "Key Structure"))
  (:`Pressed`
    (bind _asmy_game_instance (cast `MyGameInstance` (`GameplayStatics.GetGameInstance`)))
    (bind _returnvalue (`GameplayStatics.GetActorOfClass` "/Script/MyProject.Avatar"))
    (`MyGameInstance.UseItem` _asmy_game_instance _returnvalue)))

(event `self.ReceiveTick`
  (params (DeltaSeconds :type "Float (single-precision)"))
  (bind _theplayerhud (`self.ThePlayerHUD`))
  (bind _potionnumber (`/Game/JeuTripleA/Character/Paladin/Anims/Ui/WBP_PlayerHUD.PotionNumber` _theplayerhud))
  (bind _returnvalue (`self.GetGameInventory`))
  (bind _asmy_game_instance (cast `MyGameInstance` (`GameplayStatics.GetGameInstance`)))
  (if (> (`KismetArrayLibrary.Array_Length` _returnvalue) 0)
    (bind _returnvalue_2 (`MyGameInstance.GetItemInHand` _asmy_game_instance))
    (`Image.SetBrushFromTexture` (`/Game/JeuTripleA/Character/Paladin/Anims/Ui/WBP_PlayerHUD.Potions` _theplayerhud) (defaults `Object` _returnvalue_2) false)
    (bind _returnvalue_3 (`self.GetItemCount` _returnvalue_2))
    (`TextBlock.SetText` _potionnumber (`KismetTextLibrary.Conv_StringToText` (`KismetStringLibrary.Conv_IntToString` _returnvalue_3)))
    (else
      (`TextBlock.SetText` _potionnumber ""))))

(event `self.Box.OnComponentBeginOverlap`
  (params (OverlappedComponent :type "PrimitiveComponent Object Reference") (OtherActor :type "Actor Object Reference") (OtherComp :type "PrimitiveComponent Object Reference") (OtherBodyIndex :type Integer) (bFromSweep :type Boolean) (SweepResult :type "HitResult Structure (by ref)"))
  (bind _returnvalue (`GameplayStatics.GetActorOfClass` "/Script/MyProject.MyCharacter"))
  (set `MyCharacter.m_Target` OtherActor _returnvalue))

(event `self.Box.OnComponentEndOverlap`
  (params (OverlappedComponent :type "PrimitiveComponent Object Reference") (OtherActor :type "Actor Object Reference") (OtherComp :type "PrimitiveComponent Object Reference") (OtherBodyIndex :type Integer))
  (bind _returnvalue (`GameplayStatics.GetActorOfClass` "/Script/MyProject.MyCharacter"))
  (set `MyCharacter.m_Target` OtherActor _returnvalue))

(fn `UserConstructionScript`)