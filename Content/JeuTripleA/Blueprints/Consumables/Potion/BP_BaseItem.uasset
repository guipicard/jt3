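; Base world pickup actor that represents an item defined by ItemGiveClass and offers it to the player.
; On BeginPlay it constructs that item object to set its static mesh, then adds a scene component.
; Sphere overlap by BP_MyCharacter constructs a fresh item with this actor as container, prints its name and passes it to PickupSubscribe on the controller, cast to MyCharacter.
; End overlap is empty, so nothing unsubscribes here.
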(event `self.ReceiveBeginPlay`
  (bind _returnvalue (`|GenericCreateObject` (`self.ItemGiveClass`) self))
  (bind _m_mesh (`BaseItem.m_Mesh` _returnvalue))
  (bind _returnvalue_2 (`StaticMeshComponent.SetStaticMesh` (`self.StaticMesh`) _m_mesh))
  (bind _returnvalue_3 (message `MovieSceneTransformOrigin.BP_GetTransformOrigin` _m_mesh))
  (`AddComponent|NODE_AddSceneComponent-1` :`bManualAttachment` _returnvalue_2 :`RelativeTransform` _returnvalue_3))

(event `self.Sphere.OnComponentBeginOverlap`
  (params (OverlappedComponent :type "PrimitiveComponent Object Reference") (OtherActor :type "Actor Object Reference") (OtherComp :type "PrimitiveComponent Object Reference") (OtherBodyIndex :type Integer) (bFromSweep :type Boolean) (SweepResult :type "HitResult Structure (by ref)"))
  (bind _asbp_my_character (cast `/Game/JeuTripleA/Character/Paladin/BP_MyCharacter` OtherActor))
  (bind _asmy_character (cast `MyCharacter` (`Pawn.GetController` _asbp_my_character)))
  (bind _returnvalue (`|GenericCreateObject` (`self.ItemGiveClass`) self))
  (set `BaseItem.m_Container` self _returnvalue)
  (`KismetSystemLibrary.PrintString` (`KismetSystemLibrary.GetDisplayName` _returnvalue))
  (`MyCharacter.PickupSubscribe` _asmy_character _returnvalue))

(event `self.Sphere.OnComponentEndOverlap`
  (params (OverlappedComponent :type "PrimitiveComponent Object Reference") (OtherActor :type "Actor Object Reference") (OtherComp :type "PrimitiveComponent Object Reference") (OtherBodyIndex :type Integer)))

(fn `UserConstructionScript`)